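; Replay connector component that links characters to NetReplaySubsystem for socket-driven remote control of replay recording and playback.
; It binds to received commands to record, play, pause, rewind or change rate, rebinding paused when playback starts.
; Keyframes and client socket addresses relay through every BP_Character's connector to the RMI instance that issues commands.
; Debug keys trigger socket setup, RMI commands and replay, keyframe and address printouts.
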(event Custom|OnCommandRecieve
  (params (RecvCommand :type Net%20Replay%20Command%20Structure%20%28by%20ref%29))
  (bind _returnvalue (Subsystems|GetNetReplaySubsystem))
  ;[0.3017 1 0.2404] Handle commands
  (switch Utilities|FlowControl|Switch|SwitchonENetReplayCommand (.command RecvCommand)
    (:RECORD
      (Class|NetReplaySubsystem|StartRecord _returnvalue (.stringpayload RecvCommand)))
    (:STOPRECORD
      (Class|NetReplaySubsystem|StopRecording _returnvalue))
    (:PLAY
      (Class|NetReplaySubsystem|PlayNamedReplay _returnvalue (.stringpayload RecvCommand))
      (Variables|/Script/NetReplay.NetReplaySubsystem|SetbBinded _returnvalue false))
    (:PAUSE
      (bind _output_get (Variables|Default|SetIsPaused (.boolpayload RecvCommand)))
      (Class|NetReplaySubsystem|PauseReplay _returnvalue _output_get))
    (:REWINDTO
      (Class|NetReplaySubsystem|Rewindto _returnvalue (Math|Float|Truncate (.floatpayload RecvCommand))))
    (:TOSTART
      (Class|NetReplaySubsystem|Rewindto _returnvalue))
    (:RATE
      (Class|NetReplaySubsystem|ChangePlayRate _returnvalue (.floatpayload RecvCommand)))))

(event EventBeginPlay
  (bind _returnvalue (Subsystems|GetNetReplaySubsystem))
  (bind _playeruniquetype (Variables|Default|GetPlayerUniqueType))
  (bind _returnvalue_2 (Utilities|String|EnumtoString _playeruniquetype))
  ;[0.3017 1 0.2404] Handle commands
  (if (not (Networking|IsDedicatedServer))
    (Utilities|IsValid (Components|GetOwner (Components|GetOwner))
      (:Is%20Valid
        (EventDispatchers|BindEventtoOnCommandReciveDelegate _returnvalue (delegate Custom|OnCommandRecieve) :!label _label)
        (Variables|/Script/NetReplay.NetReplaySubsystem|SetbBinded _returnvalue true)
        (if (not (Utilities|Enum|Equal(Enum) _returnvalue_2 "None"))
          (Variables|/Script/NetReplay.NetReplaySubsystem|SetCharacterUniqueParam _returnvalue _returnvalue_2)))
      (:Is%20Not%20Valid
        (Utilities|Casting|CastToPlayerController (Components|GetOwner))
        (if (not (Variables|/Script/NetReplay.NetReplaySubsystem|GetbBinded _returnvalue))
          (bind _output_get (Variables|Default|SetIsPaused true))
          (Class|NetReplaySubsystem|PauseReplay _returnvalue _output_get)
          (goto _label))))))

(event Input|KeyboardEvents|DebugKey7
  (params (Key :type Key%20Structure :default "None") (ActionValue :type Input%20Action%20Value%20Structure))
  ;[1 0 0] Comment
  (:Released
    (Development|PrintString (Variables|/Script/NetReplay.NetReplaySubsystem|GetCharacterUniqueParam (Subsystems|GetNetReplaySubsystem)))))

(event Input|KeyboardEvents|DebugKey1
  (params (Key :type Key%20Structure :default "None") (ActionValue :type Input%20Action%20Value%20Structure))
  (bind _returnvalue (Subsystems|GetNetReplaySubsystem))
  ;[1 0 0] Comment
  (:Released
    (Class|NetReplaySubsystem|InitSocket _returnvalue true 1000)
    (Development|PrintString (Utilities|String|BuildString(Integer) "" "Port: " 1000))
    (Variables|/Script/NetReplay.NetReplaySubsystem|SetbRMI _returnvalue true)
    (Variables|Default|SetIsRMI true)))

(event Input|KeyboardEvents|DebugKeyNumPadFour
  (params (Key :type Key%20Structure :default "None") (ActionValue :type Input%20Action%20Value%20Structure))
  ;[1 0 0] Comment
  (:Released
    (for _array_element (Variables|/Script/NetReplay.NetReplaySubsystem|GetReplayKeyframes (Subsystems|GetNetReplaySubsystem))
      (Development|PrintString (Utilities|String|Append "Name: " (.name _array_element)))
      (Development|PrintString (Class|KismetStringLibrary|BuildStringDouble "" "Time: " (.time _array_element)))
      (Development|PrintString (Utilities|String|Append "Description: " (.description _array_element))))))

(event Input|KeyboardEvents|DebugKey2
  (params (Key :type Key%20Structure :default "None") (ActionValue :type Input%20Action%20Value%20Structure))
  ;[1 0 0] Comment
  (:Released
    (Class|NetReplaySubsystem|InitSocket (Subsystems|GetNetReplaySubsystem) false 2000)
    (Development|PrintString (Utilities|String|BuildString(Integer) "" "Port: " 2000))))

(event Input|KeyboardEvents|DebugKey3
  (params (Key :type Key%20Structure :default "None") (ActionValue :type Input%20Action%20Value%20Structure))
  ;[1 0 0] Comment
  (:Released
    (Class|NetReplaySubsystem|StartRecordingbyRMI (Subsystems|GetNetReplaySubsystem) (Variables|Default|GetCustomNameForReplay))))

(event Input|KeyboardEvents|DebugKey4
  (params (Key :type Key%20Structure :default "None") (ActionValue :type Input%20Action%20Value%20Structure))
  ;[1 0 0] Comment
  (:Released
    (Class|NetReplaySubsystem|StopRecordingbyRMI (Subsystems|GetNetReplaySubsystem))))

(event Input|KeyboardEvents|DebugKey5
  (params (Key :type Key%20Structure :default "None") (ActionValue :type Input%20Action%20Value%20Structure))
  ;[1 0 0] Comment
  (:Released
    (CallFunction|PlayReplay (Variables|/Script/NetReplay.NetReplaySubsystem|GetReplayName (Subsystems|GetNetReplaySubsystem)))))

(event Input|KeyboardEvents|DebugKey8
  (params (Key :type Key%20Structure :default "None") (ActionValue :type Input%20Action%20Value%20Structure))
  ;[1 0 0] Comment
  (:Released
    (Development|PrintString (Variables|/Script/NetReplay.NetReplaySubsystem|GetRecievedPayload (Subsystems|GetNetReplaySubsystem)))))

(event Input|KeyboardEvents|DebugKey9
  (params (Key :type Key%20Structure :default "None") (ActionValue :type Input%20Action%20Value%20Structure))
  ;[1 0 0] Comment
  (:Released
    (Class|NetReplaySubsystem|RewindtobyRMI (Subsystems|GetNetReplaySubsystem))))

(event Input|KeyboardEvents|DebugKeySubtract
  (params (Key :type Key%20Structure :default "None") (ActionValue :type Input%20Action%20Value%20Structure))
  ;[1 0 0] Comment
  (:Released
    (Class|NetReplaySubsystem|DeleteReplay (Subsystems|GetNetReplaySubsystem))))

(event Input|KeyboardEvents|6
  (params (Key :type Key%20Structure :default "None"))
  (bind _returnvalue (Subsystems|GetNetReplaySubsystem))
  ;[1 0 0] Comment
  (:Pressed
    (if (Variables|Default|GetIsPaused)
      (bind _output_get (Variables|Default|SetIsPaused false))
      (Class|NetReplaySubsystem|PauseReplaybyRMI _returnvalue _output_get)
      (else
        (bind _output_get_2 (Variables|Default|SetIsPaused true))
        (Class|NetReplaySubsystem|PauseReplaybyRMI _returnvalue _output_get_2)))))

(event Input|KeyboardEvents|0
  (params (Key :type Key%20Structure :default "None"))
  (bind _returnvalue (Subsystems|GetNetReplaySubsystem))
  ;[1 0 0] Comment
  (:Released
    (Class|NetReplaySubsystem|FindAllReplays _returnvalue)
    (Utilities|FlowControl|Delay 1.0)
    (for _array_element (Variables|/Script/NetReplay.NetReplaySubsystem|GetReplaysInfoList _returnvalue)
      (Development|PrintString (.replayname _array_element)))))

(event Input|KeyboardEvents|NumPadOne
  (params (Key :type Key%20Structure :default "None"))
  ;[1 0 0] Comment
  (:Released
    (Class|NetReplaySubsystem|ChangeFriendlyNameOfReplay (Subsystems|GetNetReplaySubsystem))))

(fn SetPause
  (params (Do%20Pause :type Boolean))
  (bind _output_get (Variables|Default|SetIsPaused Do%20Pause))
  (Class|NetReplaySubsystem|PauseReplay (Subsystems|GetNetReplaySubsystem) _output_get))

(fn PlayReplay
  (params (Replay%20Name :type String))
  (bind _returnvalue (Subsystems|GetNetReplaySubsystem))
  (Variables|/Script/NetReplay.NetReplaySubsystem|SetbBinded _returnvalue false)
  (Class|NetReplaySubsystem|PlayNamedReplaybyRMI _returnvalue Replay%20Name))

(fn AddKeyframe
  (params (Keyframe%20name :type String) (Description :type String))
  (bind _returnvalue (Subsystems|GetNetReplaySubsystem))
  (bind _returnvalue_2 (Subsystems|GetReplaySubsystem))
  (bind _returnvalue_3 (Class|ReplaySubsystem|GetReplayCurrentTime _returnvalue_2))
  (bind _replayname (Variables|/Script/NetReplay.NetReplaySubsystem|GetReplayName _returnvalue))
  (bind _keyframe (Utilities|Struct|MakeKeyframe Keyframe%20name _returnvalue_3 Description _replayname))
  (if (Class|ReplaySubsystem|IsRecording _returnvalue_2)
    (if (Variables|/Script/NetReplay.NetReplaySubsystem|GetbRMI _returnvalue)
      (Utilities|Array|Add (Variables|/Script/NetReplay.NetReplaySubsystem|GetReplayKeyframes _returnvalue) _keyframe)
      (else
        (CallFunction|SendKeyframetoServer _keyframe)))))

(event Custom|GetClientsAddresses
  (params (RMI :type BP%20Replay%20Connector%20Object%20Reference))
  ;[1 0.08476 0.7149] Collect addresses
  (bind _outactors (Actor|GetAllActorsOfClass "/Game/TestingContent/BP_Character.BP_Character_C"))
  (for _array_element _outactors
    (CallFunction|ToClient (Actor|GetComponentbyClass _array_element "BP_ReplayConnector_C") RMI)))

(event Custom|SendKeyframeToServer
  (params (Keyframe :type Keyframe%20Structure))
  ;[0.4869 0.2746 1] Keyframe RPC
  (bind _outactors (Actor|GetAllActorsOfClass "/Game/TestingContent/BP_Character.BP_Character_C"))
  (for _array_element _outactors
    (CallFunction|SendKeyframetoRMI (Actor|GetComponentbyClass _array_element "BP_ReplayConnector_C") Keyframe)))

(event Custom|ReturnToServer
  (params (RMI :type BP%20Replay%20Connector%20Object%20Reference) (IP :type Socket%20Address%20Structure))
  ;[1 0.08476 0.7149] Collect addresses
  (CallFunction|SendtoRMI RMI IP))

(event Custom|SendToRMI
  (params (Address :type Socket%20Address%20Structure))
  ;[1 0.08476 0.7149] Collect addresses
  (bind _returnvalue (Utilities|Array|Add (Variables|/Script/NetReplay.NetReplaySubsystem|GetClientsAddresses (Subsystems|GetNetReplaySubsystem)) Address))
  (Development|PrintString (Utilities|String|ToString(Integer) _returnvalue)))

(event Custom|ToClient
  (params (RMI :type BP%20Replay%20Connector%20Object%20Reference))
  (bind _returnvalue (Subsystems|GetNetReplaySubsystem))
  ;[1 0.08476 0.7149] Collect addresses
  (if (not (Variables|/Script/NetReplay.NetReplaySubsystem|GetbRMI (Subsystems|GetNetReplaySubsystem)))
    (CallFunction|ReturntoServer RMI (Utilities|Struct|MakeSocketAddress (Variables|/Script/NetReplay.NetReplaySubsystem|GetIP _returnvalue) (Variables|/Script/NetReplay.NetReplaySubsystem|GetPort _returnvalue)))))

(event Custom|SendKeyframeToRMI
  (params (Keyframe :type Keyframe%20Structure))
  (bind _returnvalue (Subsystems|GetNetReplaySubsystem))
  ;[0.4869 0.2746 1] Keyframe RPC
  (if (Variables|/Script/NetReplay.NetReplaySubsystem|GetbRMI _returnvalue)
    (Utilities|Array|Add (Variables|/Script/NetReplay.NetReplaySubsystem|GetReplayKeyframes _returnvalue) Keyframe)))

(event Input|KeyboardEvents|NumPadTwo
  (params (Key :type Key%20Structure :default "None"))
  ;[1 0.08476 0.7149] Collect addresses
  (:Released
    (CallFunction|GetClientsAddresses self)))

(event Input|KeyboardEvents|NumPadThree
  (params (Key :type Key%20Structure :default "None"))
  ;[1 0.08476 0.7149] Collect addresses
  (:Released
    (for _array_element (Variables|/Script/NetReplay.NetReplaySubsystem|GetClientsAddresses (Subsystems|GetNetReplaySubsystem))
      (Development|PrintString (.ip _array_element))
      (Development|PrintString (Utilities|String|ToString(Integer) (.port _array_element))))))