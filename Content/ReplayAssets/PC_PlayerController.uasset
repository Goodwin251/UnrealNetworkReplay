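; Player controller Blueprint that picks which character the camera views, apparently for replay playback.
; On BeginPlay it scans all BP_Character actors, skipping those whose BPReplayConnector PlayerUniqueType reads "RMI".
; It compares each remaining type, as a string, to the NetReplaySubsystem's CharacterUniqueParam and sets the first match as the view target.
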(event `self.ReceiveBeginPlay`
  (bind _outactors (`GameplayStatics.GetAllActorsOfClass` "/Game/TestingContent/BP_Character.BP_Character_C"))
  (for _array_element _outactors
    (bind _returnvalue (`|GetEnumeratorNameAsString` (`/Game/ReplayAssets/BP_ReplayConnector.PlayerUniqueType` (`/Game/TestingContent/BP_Character.BP_ReplayConnector` _array_element))))
    (if (`KismetStringLibrary.EqualEqual_StrStr` _returnvalue "RMI")
      _
      (elif (`KismetStringLibrary.EqualEqual_StrStr` _returnvalue (`NetReplaySubsystem.CharacterUniqueParam` (subsystem `NetReplaySubsystem`)))
        (`self.SetViewTargetWithBlend` _array_element)
        (break)))))

(fn `UserConstructionScript`)