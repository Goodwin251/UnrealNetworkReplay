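; BP_NetworkReplaySocket is a network socket Blueprint in the replay assets that receives strings and prints them for debugging.
; On BeginPlay it binds to its OnRecvStr delegate, storing each incoming string in RecvString and printing it.
; Releasing a debug key reprints the stored string.
; It does no parsing or replay control; the owner and BP_NetworkReplayComponent lookups are unconnected.
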(event Custom|OnRecvStr_Event
  (params (RecvStr :type String))
  (bind _output_get (Variables|Default|SetRecvString RecvStr))
  (Development|PrintString _output_get))

(event EventTick
  (params (DeltaSeconds :type Float%20%28single-precision%29)))

(event EventBeginPlay
  (EventDispatchers|AssignOnRecvStr (delegate Custom|OnRecvStr_Event)))

(event Input|KeyboardEvents|DebugKey9
  (params (Key :type Key%20Structure :default "None") (ActionValue :type Input%20Action%20Value%20Structure))
  (:Released
    (Development|PrintString (Variables|Default|GetRecvString))))