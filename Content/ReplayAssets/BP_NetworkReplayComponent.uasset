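; Character component that gathers client socket addresses for a network replay system, with debug keys for collection and replay record/playback.
; On non-server machines, BeginPlay creates and initializes a BP_NetworkReplaySocket.
; An RMI-flagged instance asks the server to poll every BP_Character's component; clients return local IP and port through the server into the requester's IPs and Ports arrays.
; ExitSocketCollecting is an empty stub; other debug keys print addresses or send a test string.
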(event Custom|RMI_Server_RequestSocketsData
  (params (RMI%20Ref :type BP%20Network%20Replay%20Component%20Object%20Reference))
  ;[0.1786 1 0.09567] Отримання айпі
  ;;[1 0.03015 0] Передати загальний клас з компонентом
  (bind _outactors (Actor|GetAllActorsOfClass "/Game/TestingContent/BP_Character.BP_Character_C"))
  (for _array_element _outactors
    (CallFunction|ServerClientCallSocketDataSend (Actor|GetComponentbyClass _array_element "BP_NetworkReplayComponent_C") RMI%20Ref))
  (CallFunction|ExitSocketCollecting))

(event Custom|RequestSocketsData
  ;[0.1786 1 0.09567] Отримання айпі
  (if (Variables|Default|GetRMI)
    (CallFunction|RMIServerRequestSocketsData self)
    (else
      (Development|PrintString "You are not RMI!" true true "(R=1.000000,G=0.033610,B=0.000000,A=1.000000)"))))

(event Custom|Server_Client_CallSocketDataSend
  (params (RMI%20Ref :type BP%20Network%20Replay%20Component%20Object%20Reference))
  ;[0.1786 1 0.09567] Отримання айпі
  (Utilities|IsValid (Variables|SocketDefaults|GetReplaySocket)
    (:Is%20Valid
      (CallFunction|ClientServerSendSocketData RMI%20Ref (Class|NetworkReplaySocket|GetLocalIP (Variables|SocketDefaults|GetReplaySocket)) (Variables|SocketDefaults|GetPort)))))

(event Custom|Client_Server_SendSocketData
  (params (RMI%20Ref :type BP%20Network%20Replay%20Component%20Object%20Reference) (IP :type String) (Port :type Integer))
  ;[0.1786 1 0.09567] Отримання айпі
  (CallFunction|ServerRMISendSocketData RMI%20Ref IP Port))

(event Custom|Server_RMI_SendSocketData
  (params (IP :type String) (Port :type Integer))
  ;[0.1786 1 0.09567] Отримання айпі
  (Utilities|Array|Add (Variables|SocketsAddresses|GetIPs) IP)
  (Utilities|Array|Add (Variables|SocketsAddresses|GetPorts) Port))

(event Custom|ExitSocketCollecting
  ;[0.1786 1 0.09567] Отримання айпі
)

(event EventBeginPlay
  ;[1 1 1] BeginPlay - створення блюпринту та інціалізація блюпринту сокета на клієнтських машинах
  (if (not (Networking|IsServer))
    (Utilities|IsValid (Components|GetOwner (Components|GetOwner))
      (:Is%20Valid
        (bind _returnvalue (Game|AddComponentbyClass (Components|GetOwner self) "/Game/ReplayAssets/BP_NetworkReplaySocket.BP_NetworkReplaySocket_C"))
        (bind _output_get (Variables|SocketDefaults|SetReplaySocket _returnvalue))
        (Class|NetworkReplaySocket|Init _output_get (Variables|Default|GetRMI) (Variables|SocketDefaults|GetPort))))))

(event Input|KeyboardEvents|DebugKey2
  (params (Key :type Key%20Structure :default "None") (ActionValue :type Input%20Action%20Value%20Structure))
  (bind _ips (Variables|SocketsAddresses|GetIPs))
  (bind _ports (Variables|SocketsAddresses|GetPorts))
  ;[1 0.03015 0] Дебаг
  (:Released
    (Development|PrintString (Utilities|String|ToString(Integer) (Utilities|Array|Length _ips)) true true "(R=0.979461,G=0.000000,B=1.000000,A=1.000000)" 1e+01)
    (Development|PrintString (Utilities|String|ToString(Integer) (Utilities|Array|Length _ports)) true true "(R=0.000000,G=0.013595,B=1.000000,A=1.000000)" 1e+01)
    (for _array_element _ips
      (Development|PrintString _array_element true true "(R=0.254941,G=1.000000,B=0.034167,A=1.000000)"))
    (for _array_element_2 _ports
      (Development|PrintString (Utilities|String|ToString(Integer) _array_element_2) true true "(R=0.000000,G=0.948892,B=1.000000,A=1.000000)"))))

(event Input|KeyboardEvents|DebugKey1
  (params (Key :type Key%20Structure :default "None") (ActionValue :type Input%20Action%20Value%20Structure))
  ;[1 0.03015 0] Виклик івенту для старту логіки запису реплея
  (:Released
    (CallFunction|RequestSocketsData)))

(event Input|KeyboardEvents|DebugKey3
  (params (Key :type Key%20Structure :default "None") (ActionValue :type Input%20Action%20Value%20Structure))
  (bind _replaysocket (Variables|SocketDefaults|GetReplaySocket))
  ;[1 0.03015 0] Дебаг
  (:Released
    (Development|PrintString (Utilities|Array|Get(acopy) (Variables|SocketsAddresses|GetIPs) 1))
    (Development|PrintString (Utilities|String|ToString(Integer) (Utilities|Array|Get(acopy) (Variables|SocketsAddresses|GetPorts) 1)))
    (Utilities|IsValid _replaysocket
      (:Is%20Valid
        (Class|NetworkReplaySocket|SendString _replaysocket "cum?" "127.0.0.1" 8800)))))

(event Input|KeyboardEvents|DebugKey4
  (params (Key :type Key%20Structure :default "None") (ActionValue :type Input%20Action%20Value%20Structure))
  (:Released
    (Class|NetworkReplayComponent|StartReplayRecord)))

(event Input|KeyboardEvents|DebugKey5
  (params (Key :type Key%20Structure :default "None") (ActionValue :type Input%20Action%20Value%20Structure))
  (:Released
    (Class|NetworkReplayComponent|StopReplayRecord)))

(event Input|KeyboardEvents|DebugKey6
  (params (Key :type Key%20Structure :default "None") (ActionValue :type Input%20Action%20Value%20Structure))
  (:Released
    (Class|NetworkReplayComponent|StartReplayPlaying)))