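; BP_Character is a test player character with basic movement, look and replay keyframe marking.
; On BeginPlay it adds an Enhanced Input mapping context, then moves relative to control rotation and applies look input to controller yaw and pitch.
; Releasing the left mouse button adds a "Click event!" keyframe through BPReplayConnector, with the current game time in its description.
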(event `self.ReceiveBeginPlay`
  ;[0 1 0.008149] Comment
  (bind _asplayer_controller (cast `PlayerController` (`self.GetController`)))
  (`EnhancedInputSubsystemInterface.AddMappingContext` (pcsubsystem `EnhancedInputLocalPlayerSubsystem` _asplayer_controller) "/Game/TestingContent/Input/IA_CharacterMapping.IA_CharacterMapping" 0 (struct)))

(event `EnhancedInput|/Game/TestingContent/Input/IA_Movement`
  (params (ActionValue :type "Vector2D Structure") (ElapsedSeconds :type "Float (double-precision)") (TriggeredSeconds :type "Float (double-precision)") (InputAction :type "InputAction Object Reference" :default "/Game/TestingContent/Input/IA_Movement.IA_Movement"))
  (bind (_returnvalue_roll _returnvalue_pitch _returnvalue_yaw) (`KismetMathLibrary.BreakRotator` (`self.GetControlRotation`)))
  ;[0 1 0.008149] Comment
  (:`Triggered`
    (`self.AddMovementInput` (`KismetMathLibrary.GetRightVector` (`KismetMathLibrary.MakeRotator` _returnvalue_roll 0.0 _returnvalue_yaw)) ActionValue_X)
    (`self.AddMovementInput` (`KismetMathLibrary.GetForwardVector` (`KismetMathLibrary.MakeRotator` 0.0 0.0 _returnvalue_yaw)) ActionValue_Y)))

(event `EnhancedInput|/Game/TestingContent/Input/IA_Look`
  (params (ActionValue :type "Vector2D Structure") (ElapsedSeconds :type "Float (double-precision)") (TriggeredSeconds :type "Float (double-precision)") (InputAction :type "InputAction Object Reference" :default "/Game/TestingContent/Input/IA_Look.IA_Look"))
  ;[0 1 0.008149] Comment
  (:`Triggered`
    (`self.AddControllerYawInput` ActionValue_X)
    (`self.AddControllerPitchInput` ActionValue_Y)))

(event `Key|LeftMouseButton`
  (params (Key :type "Key Structure"))
  ;[1 0.02238 0] Comment
  (:`Released`
    (`/Game/ReplayAssets/BP_ReplayConnector.AddKeyframe` (`self.BP_ReplayConnector`) "Click event!" (`KismetStringLibrary.BuildString_Double` "" "Happened at:  " (`GameplayStatics.GetTimeSeconds`)))))

(fn `UserConstructionScript`)